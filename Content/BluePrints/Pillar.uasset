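; Pillar obstacle actor for a Flappy Bird style game, with two pillars and a scoring box.
; On BeginPlay it shifts itself by a random height, then Tick moves it along negative X by Speed each frame, without delta-time scaling.
; A Delay in Tick destroys it after ten seconds.
; Overlapping either pillar kills the flappy player, while overlapping the box increments its Score through a DoOnce.
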(event `self.ReceiveTick`
  (params (DeltaSeconds :type "Float (single-precision)"))
  ;[1 1 1] Logic to move the pillar towards the player and destroy it after 10 seconds
  (`self.K2_SetActorLocation` (+ (`self.K2_GetActorLocation`) (`KismetMathLibrary.MakeVector` (* (`self.speed`) -1.0))))
  (`KismetSystemLibrary.Delay` 10.0)
  (`self.K2_DestroyActor`))

(event `self.Pillar1.OnComponentBeginOverlap`
  (params (OverlappedComponent :type "PrimitiveComponent Object Reference") (OtherActor :type "Actor Object Reference") (OtherComp :type "PrimitiveComponent Object Reference") (OtherBodyIndex :type Integer) (bFromSweep :type Boolean) (SweepResult :type "HitResult Structure (by ref)"))
  ;[1 1 1] Logic to kill the player if overlaped with the pillar
  (bind _asflappy (cast `/Game/BluePrints/flappy` OtherActor))
  (`/Game/BluePrints/flappy.Kill Player` _asflappy))

(event `self.ReceiveBeginPlay`
  ;[1 1 1] Logic to spawn the player in a random Z location in range
  (`self.K2_SetActorLocation` (+ (`self.K2_GetActorLocation`) (`KismetMathLibrary.MakeVector` 0.0 0.0 (`KismetMathLibrary.RandomFloatInRange` -400.0 400.0)))))

(event `self.Box.OnComponentBeginOverlap`
  (params (OverlappedComponent :type "PrimitiveComponent Object Reference") (OtherActor :type "Actor Object Reference") (OtherComp :type "PrimitiveComponent Object Reference") (OtherBodyIndex :type Integer) (bFromSweep :type Boolean) (SweepResult :type "HitResult Structure (by ref)"))
  ;[1 1 1] Logic to increment the player Score if overlaped with the Collision Box
  (bind _asflappy (cast `/Game/BluePrints/flappy` OtherActor))
  (`/Engine/EditorBlueprintResources/StandardMacros.DoOnce` false
    (:`Completed`
      (bind _result (`/Engine/EditorBlueprintResources/StandardMacros.IncrementInt` (`/Game/BluePrints/flappy.Score` _asflappy))
        (:`  `
          (set `/Game/BluePrints/flappy.Score` _result _asflappy))))))

(event `self.Pillar 2.OnComponentBeginOverlap`
  (params (OverlappedComponent :type "PrimitiveComponent Object Reference") (OtherActor :type "Actor Object Reference") (OtherComp :type "PrimitiveComponent Object Reference") (OtherBodyIndex :type Integer) (bFromSweep :type Boolean) (SweepResult :type "HitResult Structure (by ref)"))
  ;[1 1 1] Logic to kill the player if overlaped with the pillar
  (bind _asflappy (cast `/Game/BluePrints/flappy` OtherActor))
  (`/Game/BluePrints/flappy.Kill Player` _asflappy))

(fn `UserConstructionScript`)