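; Player Blueprint for a Flappy Bird-style game, handling jumping, death and level restart.
; Space applies an upward force to the physics-driven Player component until IsDead is set, and E reopens MainLevel at any time.
; KillPlayer sets that flag and knocks the body away with an angular impulse and a force as a death animation.
; BeginPlay adds the Score widget to the viewport.
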(event `self.ReceiveTick`
  (params (DeltaSeconds :type "Float (single-precision)")))

(event `Key|SpaceBar`
  (params (Key :type "Key Structure"))
  ;[1 1 1] Jumping Logic
  (:`Pressed`
    (if (not (`self.is dead`))
      (`PrimitiveComponent.AddForce` (`self.Player`) (0.0 0.0 30000.0) "None" false))))

(event `self.ReceiveBeginPlay`
  ;[1 1 1] adding the score counter to screen
  (bind _returnvalue (`|CreateWidget` "/Game/Widgets/Score.Score_C"))
  (`UserWidget.AddToViewport` _returnvalue 0))

(event `Key|E`
  (params (Key :type "Key Structure"))
  ;[1 1 1] Logic to Help Restart the level
  (:`Pressed`
    (`GameplayStatics.OpenLevel` "MainLevel")))

(fn `Kill Player`
  (bind _player (`self.Player`))
  ;[1 1 1] death logic and death animation
  (set `self.is dead` true)
  (`PrimitiveComponent.AddAngularImpulseInDegrees` _player (0.0 -5000000.0 0.0) "None" false)
  (`PrimitiveComponent.AddForce` _player (-300000.0 0.0 300000.0) "None" false))

(fn `UserConstructionScript`)